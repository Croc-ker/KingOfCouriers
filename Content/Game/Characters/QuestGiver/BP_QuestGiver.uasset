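; BP_QuestGiver is a quest NPC that shows dialogue and accepts a wanted item from the player.
; Each Talk call advances through the Speech array in a WBP_SpeechBox with portrait, blending the camera to the NPC and flagging BP_DD as Talking.
; After the last line it removes the box, resets and returns the camera.
; On overlap, it removes a matching held pickup by name and switches Speech to FoundSpeech.
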(event `/Game/Game/Characters/QuestGiver/BPI_Dialogue.Talk`
  (bind _speechindex (`self.SpeechIndex`))
  (bind _ui (`self.UI`))
  (`PlayerController.SetViewTargetWithBlend` (`GameplayStatics.GetPlayerController` 0) self 0.5 "VTBlend_Linear" 0.0 false)
  (bind _asbp_dd (cast `/Game/Game/Characters/DD/BP_DD` (`GameplayStatics.GetPlayerCharacter` 0)))
  (set `/Game/Game/Characters/DD/BP_DD.Talking` true _asbp_dd)
  (`/Engine/EditorBlueprintResources/StandardMacros.IncrementInt` _speechindex
    (:`  `
      (if (< _speechindex (`KismetArrayLibrary.Array_Length` (`self.Speech`)))
        (`self.UI`
          (:`then`
            _)
          (:`else`
            (bind _returnvalue (`|CreateWidget` "/Game/Game/UI/WBP_SpeechBox.WBP_SpeechBox_C" (`GameplayStatics.GetPlayerController` 0)))
            (bind _output_get (set `self.UI` _returnvalue))
            (`UserWidget.AddToViewport` _output_get 0)))
        (`TextBlock.SetText` (`/Game/Game/UI/WBP_SpeechBox.TalkText` _ui) (`KismetTextLibrary.Conv_StringToText` (`|GetArrayItem` (`self.Speech`) (`self.SpeechIndex`))))
        (`Image.SetBrushFromTexture` (`/Game/Game/UI/WBP_SpeechBox.Portrait` _ui) (`self.PortraitTex`) false)
        (else
          (`Widget.RemoveFromParent` (`self.UI`))
          (bind _asbp_dd_2 (cast `/Game/Game/Characters/DD/BP_DD` (`GameplayStatics.GetPlayerCharacter` 0)))
          (set `/Game/Game/Characters/DD/BP_DD.Talking` false _asbp_dd_2)
          (`PlayerController.SetViewTargetWithBlend` (`GameplayStatics.GetPlayerController` 0) (`GameplayStatics.GetPlayerCharacter` 0) 0.5 "VTBlend_Linear" 0.0 false)
          (set `self.SpeechIndex` -1)
          (set `self.UI` null))))))

(event `self.ReceiveActorBeginOverlap`
  (params (OtherActor :type "Actor Object Reference"))
  (`self.PlayerHasItem` OtherActor))

(fn `PlayerHasItem`
  (params (Object :type "Object Object Reference"))
  (bind _asbp_dd (cast `/Game/Game/Characters/DD/BP_DD` Object))
  (bind _heldpickups (`/Game/Game/Characters/DD/BP_DD.HeldPickups` _asbp_dd))
  (for _array_element _heldpickups
    (`/Engine/EditorBlueprintResources/StandardMacros.IsValid` _array_element
      (:`Is Valid`
        (if (`KismetStringLibrary.EqualEqual_StrStr` (`/Game/Game/Objects/Pickupable/BP_Pickup.Name` _array_element) (`self.WantedItem`))
          (`KismetArrayLibrary.Array_RemoveItem` _heldpickups _array_element)
          (set `self.Speech` (`self.FoundSpeech`))
          (break))))))

(fn `UserConstructionScript`)