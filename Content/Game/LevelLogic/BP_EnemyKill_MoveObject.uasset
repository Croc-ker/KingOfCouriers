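; Level-logic actor that moves a referenced Object to the ObjectMoveEnd actor's location once every listed enemy is gone.
; Tick removes invalid entries from the Enemies array by polling, with no death events.
; With the array empty, MoveObject runs every frame, either teleporting the Object or easing it over with VInterpTo, depending on the Teleport flag.
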(event `self.ReceiveTick`
  (params (DeltaSeconds :type "Float (single-precision)"))
  (if (> (`KismetArrayLibrary.Array_Length` (`self.Enemies`)) 0)
    (for _array_element (`self.Enemies`)
      (`/Engine/EditorBlueprintResources/StandardMacros.IsValid` _array_element
        (:`Is Not Valid`
          (`KismetArrayLibrary.Array_RemoveItem` (`self.Enemies`) _array_element))))
    (else
      (`self.MoveObject` (`self.Teleport`)))))

(fn `MoveObject`
  (params (Teleport :type Boolean))
  (bind _object (`self.Object`))
  (if Teleport
    (`self.K2_SetActorLocation` (`self.Object`) (`self.K2_GetActorLocation` (`self.ObjectMoveEnd`)) false true)
    (else
      (`self.K2_SetActorLocation` _object (`KismetMathLibrary.VInterpTo` (`self.K2_GetActorLocation` _object) (`self.K2_GetActorLocation` (`self.ObjectMoveEnd`)) (`GameplayStatics.GetWorldDeltaSeconds`) 1.0) false false))))

(fn `UserConstructionScript`)