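; BP_Gunbot is the Gunbot enemy Blueprint, whose graph handles only taking damage and dying.
; AnyDamage subtracts from Health and, at zero or below, reports a "Robot" kill with its Multiplier to the CourierGameInstance combo system before destroying the actor.
; Destruction follows the game instance cast, so it is skipped if that cast fails.
; BeginPlay, overlap and Tick are disabled stubs, and the construction script only calls its parent.
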(event `self.ReceiveAnyDamage`
  (params (Damage :type "Float (single-precision)") (DamageType :type "DamageType Object Reference") (InstigatedBy :type "Controller Object Reference") (DamageCauser :type "Actor Object Reference"))
  (bind _output_get (set `self.Health` (- (`self.Health`) Damage)))
  (if (<= _output_get 0.0)
    (bind _ascourier_game_instance (cast `/Game/Game/CourierGameInstance` (`GameplayStatics.GetGameInstance`)))
    (`/Game/Game/CourierGameInstance.AddCombo` _ascourier_game_instance "Robot" (`self.Multiplier`))
    (`self.K2_DestroyActor`)))

(fn `UserConstructionScript`
  (`parent.UserConstructionScript`))