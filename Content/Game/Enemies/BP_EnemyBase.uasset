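; BP_EnemyBase is an enemy base Blueprint whose bleed damage, attack and movement permissions are driven by a beat.
; OnBeat applies bleed damage credited to the player while Bleeding, then re-enables CanAttack and CanMove.
; It also mirrors CanAttack to the Blackboard's Attack key when a Blackboard is valid.
; On destruction, the enemy removes itself from the CourierGameMode Enemies list.
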(event `self.ReceiveDestroyed`
  (bind _ascourier_game_mode (cast `/Game/Game/CourierGameMode` (`GameplayStatics.GetGameMode`)))
  (`KismetArrayLibrary.Array_RemoveItem` (`/Game/Game/CourierGameMode.Enemies` _ascourier_game_mode) self))

(fn `OnBeat`
  (bind _returnvalue (`AIBlueprintHelperLibrary.GetBlackboard` null))
  (`|ExecutionSequence`
    (:`then_0`
      (if (`self.Bleeding`)
        (`GameplayStatics.ApplyDamage` self 10.0 (`GameplayStatics.GetPlayerController` 0) (`GameplayStatics.GetPlayerCharacter` 0))))
    (:`then_1`
      (bind _output_get (set `self.CanAttack` true))
      (`/Engine/EditorBlueprintResources/StandardMacros.IsValid` _returnvalue
        (:`Is Valid`
          (`BlackboardComponent.SetValueAsBool` _returnvalue (`self.Attack?`) _output_get))))
    (:`then_2`
      (set `self.CanMove` true))))

(fn `UserConstructionScript`)