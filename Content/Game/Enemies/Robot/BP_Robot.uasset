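; BP_Robot is a robot enemy that hurts the player on contact and awards a combo when killed.
; Tick checks the first BP_DD overlapping its capsule for the Player tag, then uses a DoOnce and Delay to apply damage about once per second.
; AnyDamage reduces Health, and at zero it reports the kill and multiplier to CourierGameInstance before destroying itself.
; A separate AddScore function increments the game instance's Score but is not called here.
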(event `self.ReceiveActorBeginOverlap`
  (params (OtherActor :type "Actor Object Reference")))

(event `self.ReceiveTick`
  (params (DeltaSeconds :type "Float (single-precision)"))
  (bind _output (`|GetArrayItem` (`PrimitiveComponent.GetOverlappingActors` (`self.Capsule`) "/Game/Game/Characters/DD/BP_DD.BP_DD_C")))
  (`/Engine/EditorBlueprintResources/StandardMacros.IsValid` _output
    (:`Is Valid`
      (if (`self.ActorHasTag` _output "Player")
        (`/Engine/EditorBlueprintResources/StandardMacros.DoOnce` false :!label _label
          (:`Completed`
            (`KismetSystemLibrary.Delay` 1.0)
            (`GameplayStatics.ApplyDamage` _output 34.0 (`AIBlueprintHelperLibrary.GetAIController` self) self)
            (goto _label :!via `Reset`)))))))

(event `self.ReceiveAnyDamage`
  (params (Damage :type "Float (single-precision)") (DamageType :type "DamageType Object Reference") (InstigatedBy :type "Controller Object Reference") (DamageCauser :type "Actor Object Reference"))
  (bind _output_get (set `self.Health` (- (`self.Health`) Damage)))
  (if (<= _output_get 0.0)
    (bind _ascourier_game_instance (cast `/Game/Game/CourierGameInstance` (`GameplayStatics.GetGameInstance`)))
    (`/Game/Game/CourierGameInstance.AddCombo` _ascourier_game_instance "Robot" (`self.Multiplier`))
    (`self.K2_DestroyActor`)))

(fn `AddScore`
  (bind _ascourier_game_instance (cast `/Game/Game/CourierGameInstance` (`GameplayStatics.GetGameInstance`)))
  (bind _result (`/Engine/EditorBlueprintResources/StandardMacros.IncrementInt` (`/Game/Game/CourierGameInstance.Score` _ascourier_game_instance))
    (:`  `
      (set `/Game/Game/CourierGameInstance.Score` _result _ascourier_game_instance))))

(fn `UserConstructionScript`)