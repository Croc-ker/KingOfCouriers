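; BP_Turret is an enemy turret that fires continuously and can be destroyed for combo points.
; Tick drives a DoOnce that spawns BP_EnemyBullet at the Barrel's transform with a rotation offset, then resets after a short Delay to set the fire rate.
; AnyDamage reduces health, and at zero reports a Turret combo with its multiplier to CourierGameInstance before destroying the actor.
; A separate AddScore function increments the game instance's Score.
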(event `self.ReceiveActorBeginOverlap`
  (params (OtherActor :type "Actor Object Reference")))

(event `self.ReceiveTick`
  (params (DeltaSeconds :type "Float (single-precision)"))
  (bind (_returnvalue_location _returnvalue_rotation _returnvalue_scale) (`KismetMathLibrary.BreakTransform` (`SceneComponent.K2_GetComponentToWorld` (`self.Barrel`))))
  (`/Engine/EditorBlueprintResources/StandardMacros.DoOnce` false :!label _label
    (:`Completed`
      (`|SpawnActorFromClass` "/Game/Game/Enemies/Turret/BP_EnemyBullet.BP_EnemyBullet_C" (`KismetMathLibrary.MakeTransform` _returnvalue_location (`KismetMathLibrary.ComposeRotators` _returnvalue_rotation (struct :`Yaw` 90.0)) _returnvalue_scale) "Undefined" "MultiplyWithRoot" null null)
      (`KismetSystemLibrary.Delay` 0.8)
      (goto _label :!via `Reset`))))

(event `self.ReceiveAnyDamage`
  (params (Damage :type "Float (single-precision)") (DamageType :type "DamageType Object Reference") (InstigatedBy :type "Controller Object Reference") (DamageCauser :type "Actor Object Reference"))
  (set `self.Health_0` (- (`self.Health_0`) Damage))
  (if (<= (`self.Health_0`) 0.0)
    (bind _ascourier_game_instance (cast `/Game/Game/CourierGameInstance` (`GameplayStatics.GetGameInstance`)))
    (`/Game/Game/CourierGameInstance.AddCombo` _ascourier_game_instance "Turret" (`self.Multiplier`))
    (`self.K2_DestroyActor`)))

(fn `AddScore`
  (bind _ascourier_game_instance (cast `/Game/Game/CourierGameInstance` (`GameplayStatics.GetGameInstance`)))
  (bind _result (`/Engine/EditorBlueprintResources/StandardMacros.IncrementInt` (`/Game/Game/CourierGameInstance.Score` _ascourier_game_instance))
    (:`  `
      (set `/Game/Game/CourierGameInstance.Score` _result _ascourier_game_instance))))

(fn `UserConstructionScript`)