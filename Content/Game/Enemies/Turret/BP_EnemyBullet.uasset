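; Enemy projectile that damages the player and can be knocked back to damage enemies, with a short lifespan.
; Damage from a non-enemy causer tags it Reflected, plays a pitch-varied ricochet and redirects it toward the nearest BP_EnemyBase in range, otherwise reversing its velocity.
; Overlaps use Player, Enemy and Reflected tags to choose valid targets.
; An unreflected bullet destroys itself on overlapping a Reflected actor.
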(event `self.ReceiveBeginPlay`
  (`self.SetLifeSpan` 5.0))

(event `self.ReceiveActorBeginOverlap`
  (params (OtherActor :type "Actor Object Reference"))
  (bind _returnvalue (`self.ActorHasTag` "Reflected"))
  (`/Engine/EditorBlueprintResources/StandardMacros.IsValid` OtherActor
    (:`Is Valid`
      (if (or (and (`self.ActorHasTag` OtherActor "Player") (not _returnvalue)) (and _returnvalue (`self.ActorHasTag` OtherActor "Enemy")))
        (`/Engine/EditorBlueprintResources/StandardMacros.IsValid` OtherActor
          (:`Is Valid`
            (`GameplayStatics.ApplyDamage` OtherActor 15.0 null self))))
      (`/Engine/EditorBlueprintResources/StandardMacros.IsValid` OtherActor
        (:`Is Valid`
          (if (and (not (`self.ActorHasTag` "Reflected")) (`self.ActorHasTag` OtherActor "Reflected"))
            (`self.K2_DestroyActor`)))))))

(event `self.ReceiveAnyDamage`
  (params (Damage :type "Float (single-precision)") (DamageType :type "DamageType Object Reference") (InstigatedBy :type "Controller Object Reference") (DamageCauser :type "Actor Object Reference"))
  (bind _returnvalue (`self.K2_GetActorLocation`))
  (bind _projectilemovement (`self.ProjectileMovement`))
  (`/Engine/EditorBlueprintResources/StandardMacros.IsValid` DamageCauser
    (:`Is Valid`
      (if (not (`self.ActorHasTag` DamageCauser "Enemy"))
        (`GameplayStatics.PlaySoundAtLocation` "/Game/Game/Sounds/physical/Ricochet.Ricochet" _returnvalue (struct) 1.0 (`KismetMathLibrary.RandomFloatInRange` 0.9 1.1) 0.0 null null null null)
        (`KismetArrayLibrary.Array_Add` (`self.Tags`) "Reflected")
        (bind _outactors (`GameplayStatics.GetAllActorsOfClass` "/Game/Game/Enemies/BP_EnemyBase.BP_EnemyBase_C"))
        (bind (_distance _returnvalue_2) (`GameplayStatics.FindNearestActor` _returnvalue _outactors))
        (if (<= _distance 2000.0)
          (set `MovementComponent.Velocity` (* (`KismetMathLibrary.GetForwardVector` (`KismetMathLibrary.FindLookAtRotation` _returnvalue (`self.K2_GetActorLocation` _returnvalue_2))) 1000.0) (`self.ProjectileMovement`))
          (else
            (set `MovementComponent.Velocity` (* (`MovementComponent.Velocity` _projectilemovement) -1.0) _projectilemovement)))))))

(fn `UserConstructionScript`)