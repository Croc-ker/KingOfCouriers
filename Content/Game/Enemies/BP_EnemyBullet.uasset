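; BP_EnemyBullet is an enemy projectile that damages actors tagged Player on overlap, then destroys itself, and otherwise expires after a short lifespan.
; Taking any damage deflects it and adds a Reflected tag.
; On deflection it aims its Sphere at the nearest BP_Robot and launches straight at it if one is close enough, otherwise it reverses its velocity at double speed.
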(event `self.ReceiveBeginPlay`
  (`self.SetLifeSpan` 5.0))

(event `self.ReceiveActorBeginOverlap`
  (params (OtherActor :type "Actor Object Reference"))
  (if (`self.ActorHasTag` OtherActor "Player")
    (`GameplayStatics.ApplyDamage` OtherActor 25.0 null self)
    (`self.K2_DestroyActor`)))

(event `self.ReceiveAnyDamage`
  (params (Damage :type "Float (single-precision)") (DamageType :type "DamageType Object Reference") (InstigatedBy :type "Controller Object Reference") (DamageCauser :type "Actor Object Reference"))
  (bind _projectilemovement (`self.ProjectileMovement`))
  (bind _returnvalue (`SceneComponent.K2_GetComponentLocation` (`self.Sphere`)))
  (`KismetArrayLibrary.Array_Add` (`self.Tags`) "Reflected")
  (bind _outactors (`GameplayStatics.GetAllActorsOfClass` "/Game/Game/Enemies/Robot/BP_Robot.BP_Robot_C"))
  (bind (_distance _returnvalue_2) (`GameplayStatics.FindNearestActor` _returnvalue _outactors))
  (if (<= _distance 500.0)
    (`SceneComponent.K2_SetWorldRotation` (`self.Sphere`) (`KismetMathLibrary.FindLookAtRotation` _returnvalue (`self.K2_GetActorLocation` _returnvalue_2)) false false)
    (set `MovementComponent.Velocity` (* (`SceneComponent.GetForwardVector` (`self.Sphere`)) 2000.0) _projectilemovement)
    (else
      (set `MovementComponent.Velocity` (* (`MovementComponent.Velocity` _projectilemovement) -2.0) _projectilemovement))))

(fn `UserConstructionScript`)