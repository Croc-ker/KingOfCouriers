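; BP_Mailbox is a delivery point that completes a mail delivery when the BP_DD character overlaps it.
; It records its name on the character, snaps them to its arrow and plays a delivery montage with input disabled and two timed camera cuts, then restores control and destroys itself.
; The overlap also refills Health and checks the matching mail list entry by name.
; An unconnected Mail-tag scoring branch never runs.
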(event `self.ReceiveActorBeginOverlap`
  (params (OtherActor :type "Actor Object Reference"))
  (bind _returnvalue (`GameplayStatics.GetPlayerController` 0))
  (bind (_returnvalue_location _returnvalue_rotation) (`KismetMathLibrary.BreakTransform` (`SceneComponent.K2_GetComponentToWorld` (`self.Arrow`))))
  (`|ExecutionSequence`
    (:`then_0`
      (bind _asbp_dd (cast `/Game/Game/Characters/DD/BP_DD` OtherActor))
      (`KismetArrayLibrary.Array_Add` (`/Game/Game/Characters/DD/BP_DD.MailboxesGotten` _asbp_dd) (`self.Name`))
      (set `MovementComponent.Velocity` (0.0 0.0 0.0) (`Character.CharacterMovement` _asbp_dd))
      (`self.K2_SetActorTransform` _asbp_dd (`KismetMathLibrary.MakeTransform` _returnvalue_location _returnvalue_rotation) false false)
      (set `/Game/Game/Characters/DD/BP_DD.LookAt` false _asbp_dd)
      (`self.DisableInput` _asbp_dd (`GameplayStatics.GetPlayerController` 0))
      (`self.DisableInput` (`GameplayStatics.GetPlayerController` 0) (`GameplayStatics.GetPlayerController` 0))
      (`self.DisableInput` (`GameplayStatics.GetPlayerCharacter` 0) (`GameplayStatics.GetPlayerController` 0))
      (`|PlayMontage` (`Character.Mesh` _asbp_dd) "/Game/Game/Characters/DD/Animations/MailboxDeliver_Montage.MailboxDeliver_Montage"
        (:`then`
          (`ActorComponent.Deactivate` (`/Game/Game/Characters/DD/BP_DD.Camera` _asbp_dd))
          (bind _mailboxcam1 (`/Game/Game/Characters/DD/BP_DD.MailboxCam1` _asbp_dd))
          (`ActorComponent.SetActive` _mailboxcam1 true false)
          (`KismetSystemLibrary.Delay` 0.79)
          (`ActorComponent.Deactivate` _mailboxcam1)
          (`ActorComponent.SetActive` (`/Game/Game/Characters/DD/BP_DD.MailboxCam2` _asbp_dd) true false)
          (`KismetSystemLibrary.Delay` 2.0)
          (`ActorComponent.Deactivate` (`/Game/Game/Characters/DD/BP_DD.MailboxCam1` _asbp_dd))
          (`ActorComponent.Deactivate` (`/Game/Game/Characters/DD/BP_DD.MailboxCam2` _asbp_dd))
          (`ActorComponent.SetActive` (`/Game/Game/Characters/DD/BP_DD.Camera` _asbp_dd) true false)
          (set `/Game/Game/Characters/DD/BP_DD.LookAt` true _asbp_dd)
          (`self.EnableInput` _returnvalue _returnvalue)
          (`self.EnableInput` (`GameplayStatics.GetPlayerCharacter` 0) _returnvalue)
          (`Character.StopAnimMontage` _asbp_dd "/Game/Game/Characters/DD/Animations/MailboxDeliver_Montage.MailboxDeliver_Montage")
          (`self.K2_DestroyActor`))))
    (:`then_1`
      (bind _asbp_dd_2 (cast `/Game/Game/Characters/DD/BP_DD` OtherActor))
      (set `/Game/Game/Characters/DD/BP_DD.Health` 100.0 _asbp_dd_2)
      (for _array_element (`PanelWidget.GetAllChildren` (`/Game/Game/UI/WBP_MailList.BoxList` (`/Game/Game/Characters/DD/BP_DD.MailListUI` _asbp_dd_2)))
        (bind _aswbp_mail_list_box (cast `/Game/Game/UI/WBP_MailList_Box` _array_element))
        (if (== (`/Game/Game/UI/WBP_MailList_Box.Name` _aswbp_mail_list_box) (`self.Name`))
          (`CheckBox.SetCheckedState` (`/Game/Game/UI/WBP_MailList_Box.DoneBox` _aswbp_mail_list_box) "Checked"))))))

(fn `UserConstructionScript`)