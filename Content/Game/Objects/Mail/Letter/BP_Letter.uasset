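; BP_Letter is a short-lived mail letter actor that can be delivered or can hurt what it touches.
; It expires after a fixed lifespan, is destroyed by any damage, and ignores overlaps with Player-tagged actors.
; Overlapping a Delivery-tagged actor destroys it after a tiny delay.
; Any other valid actor takes damage, with BP_EnemyBase targets also set Bleeding, and the letter destroys itself.
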(event `self.ReceiveBeginPlay`
  (`self.SetLifeSpan` 10.0))

(event `self.ReceiveActorBeginOverlap`
  (params (OtherActor :type "Actor Object Reference"))
  (`/Engine/EditorBlueprintResources/StandardMacros.IsValid` OtherActor
    (:`Is Valid`
      (if (`self.ActorHasTag` OtherActor "Player")
        _
        (elif (`self.ActorHasTag` OtherActor "Delivery")
          (`KismetSystemLibrary.Delay` 0.01)
          (`self.K2_DestroyActor`)
          (else
            (`GameplayStatics.ApplyDamage` OtherActor 50.0 null self)
            (bind _asbp_enemy_base (cast `/Game/Game/Enemies/BP_EnemyBase` OtherActor)
              (:`then`
                _)
              (:`CastFailed`
                _))
            (`/Engine/EditorBlueprintResources/StandardMacros.IsValid` _asbp_enemy_base
              (:`Is Valid`
                (set `/Game/Game/Enemies/BP_EnemyBase.Bleeding` true _asbp_enemy_base))
              (:`Is Not Valid`
                _))
            (`self.K2_DestroyActor`)))))))

(event `self.ReceiveAnyDamage`
  (params (Damage :type "Float (single-precision)") (DamageType :type "DamageType Object Reference") (InstigatedBy :type "Controller Object Reference") (DamageCauser :type "Actor Object Reference"))
  (`self.K2_DestroyActor`))

(fn `UserConstructionScript`)