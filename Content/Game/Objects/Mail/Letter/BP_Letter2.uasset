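; BP_Letter2 is a short-lived mail letter actor that damages what it overlaps and expires on its own after a set lifespan.
; Until tagged Reflected or Thrown, Tick moves its Cube to the X and Y of the BP_DD player's Pointer, keeping its own height.
; Overlapping a Delivery or Player actor destroys it harmlessly after a tiny delay, other actors take damage as it is destroyed, and any damage received also destroys it.
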(event `self.ReceiveBeginPlay`
  (`self.SetLifeSpan` 10.0))

(event `self.ReceiveActorBeginOverlap`
  (params (OtherActor :type "Actor Object Reference"))
  (`/Engine/EditorBlueprintResources/StandardMacros.IsValid` OtherActor
    (:`Is Valid`
      (if (or (`self.ActorHasTag` OtherActor "Delivery") (`self.ActorHasTag` OtherActor "Player"))
        (`KismetSystemLibrary.Delay` 0.01)
        (`self.K2_DestroyActor`)
        (else
          (`GameplayStatics.ApplyDamage` OtherActor 50.0 null self)
          (`self.K2_DestroyActor`))))))

(event `self.ReceiveTick`
  (params (DeltaSeconds :type "Float (single-precision)"))
  (bind (_returnvalue_x _returnvalue_y _returnvalue_z) (`KismetMathLibrary.BreakVector` (`SceneComponent.K2_GetComponentLocation` (`self.Cube`))))
  (if (not (or (`self.ActorHasTag` "Reflected") (`self.ActorHasTag` "Thrown")))
    (bind _asbp_dd (cast `/Game/Game/Characters/DD/BP_DD` (`GameplayStatics.GetPlayerCharacter` 0)))
    (bind (_returnvalue_x_2 _returnvalue_y_2) (`KismetMathLibrary.BreakVector` (`SceneComponent.K2_GetComponentLocation` (`/Game/Game/Characters/DD/BP_DD.Pointer` _asbp_dd))))
    (`SceneComponent.K2_SetWorldLocation` (`self.Cube`) (`KismetMathLibrary.MakeVector` _returnvalue_x_2 _returnvalue_y_2 _returnvalue_z) false false)))

(event `self.ReceiveAnyDamage`
  (params (Damage :type "Float (single-precision)") (DamageType :type "DamageType Object Reference") (InstigatedBy :type "Controller Object Reference") (DamageCauser :type "Actor Object Reference"))
  (`self.K2_DestroyActor`))

(fn `UserConstructionScript`)