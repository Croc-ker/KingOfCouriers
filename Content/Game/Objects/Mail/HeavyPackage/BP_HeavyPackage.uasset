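; Heavy package projectile that expires after ten seconds and vanishes shortly after overlapping a Delivery-tagged actor.
; Until tagged Reflected or Thrown, its cube follows the XY position of the BP_DD player's Pointer every tick.
; Without its own Mail tag, it damages other overlapped actors and destroys itself.
; Damage from a Player-tagged causer launches it forward and slightly upward, then runs the parent Reflect.
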(event `self.ReceiveBeginPlay`
  (`self.SetLifeSpan` 10.0))

(event `self.ReceiveActorBeginOverlap`
  (params (OtherActor :type "Actor Object Reference"))
  (`/Engine/EditorBlueprintResources/StandardMacros.IsValid` OtherActor
    (:`Is Valid`
      (if (`self.ActorHasTag` OtherActor "Delivery")
        (`KismetSystemLibrary.Delay` 0.01)
        (`self.K2_DestroyActor`)
        (elif (not (`self.ActorHasTag` "Mail"))
          (`GameplayStatics.ApplyDamage` OtherActor 100.0 null self)
          (`self.K2_DestroyActor`))))))

(event `self.ReceiveTick`
  (params (DeltaSeconds :type "Float (single-precision)"))
  (bind (_returnvalue_x _returnvalue_y _returnvalue_z) (`KismetMathLibrary.BreakVector` (`SceneComponent.K2_GetComponentLocation` (`self.Cube`))))
  (if (not (or (`self.ActorHasTag` "Reflected") (`self.ActorHasTag` "Thrown")))
    (bind _asbp_dd (cast `/Game/Game/Characters/DD/BP_DD` (`GameplayStatics.GetPlayerCharacter` 0)))
    (bind (_returnvalue_x_2 _returnvalue_y_2) (`KismetMathLibrary.BreakVector` (`SceneComponent.K2_GetComponentLocation` (`/Game/Game/Characters/DD/BP_DD.Pointer` _asbp_dd))))
    (`SceneComponent.K2_SetWorldLocation` (`self.Cube`) (`KismetMathLibrary.MakeVector` _returnvalue_x_2 _returnvalue_y_2 _returnvalue_z) false false)))

(event `self.ReceiveAnyDamage`
  (params (Damage :type "Float (single-precision)") (DamageType :type "DamageType Object Reference") (InstigatedBy :type "Controller Object Reference") (DamageCauser :type "Actor Object Reference"))
  (`/Engine/EditorBlueprintResources/StandardMacros.IsValid` DamageCauser
    (:`Is Valid`
      (if (`self.ActorHasTag` DamageCauser "Player")
        (`self.Reflect` DamageCauser)))))

(fn `Reflect`
  (params (DamageCauser :type "Actor Object Reference"))
  (set `MovementComponent.Velocity` (* (+ (`self.GetActorForwardVector` DamageCauser) (0.0 0.0 0.25)) 2000.0) (`self.ProjectileMovement`))
  (`parent.Reflect` DamageCauser))

(fn `UserConstructionScript`)