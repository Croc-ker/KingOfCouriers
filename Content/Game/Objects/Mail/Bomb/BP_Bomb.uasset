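; BP_Bomb is a mail-object bomb that explodes on overlap, dealing full radial damage while sparing the player, and expires on a timer.
; Overlapping a Delivery-tagged actor instead destroys it without exploding.
; Until tagged Thrown or Reflected, Tick keeps its Cube at the XY of BP_DD's Pointer.
; Damage caused by a Player-tagged actor launches it along that actor's forward vector with slight lift, then calls parent Reflect.
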(event `self.ReceiveBeginPlay`
  (`self.SetLifeSpan` 10.0))

(event `self.ReceiveActorBeginOverlap`
  (params (OtherActor :type "Actor Object Reference"))
  (bind _returnvalue (`self.K2_GetActorLocation`))
  (bind _array (`|MakeArray` (`GameplayStatics.GetPlayerCharacter` 0) :!type "Actor Object Reference"))
  (`/Engine/EditorBlueprintResources/StandardMacros.IsValid` OtherActor
    (:`Is Valid`
      (if (`self.ActorHasTag` OtherActor "Delivery")
        (`KismetSystemLibrary.Delay` 0.01)
        (`self.K2_DestroyActor`)
        (else
          (`GameplayStatics.ApplyRadialDamage` 500.0 _returnvalue 600.0 null _array self (`GameplayStatics.GetPlayerController` 0) true "ECC_WorldStatic")
          (`KismetSystemLibrary.SphereTraceSingleForObjects` _returnvalue _returnvalue 600.0 (`|MakeArray` "ObjectTypeQuery3" :!type "EObjectTypeQuery Enum") false _array "ForOneFrame")
          (`self.K2_DestroyActor`))))))

(event `self.ReceiveTick`
  (params (DeltaSeconds :type "Float (single-precision)"))
  (bind (_returnvalue_x _returnvalue_y _returnvalue_z) (`KismetMathLibrary.BreakVector` (`SceneComponent.K2_GetComponentLocation` (`self.Cube`))))
  (if (not (or (`self.ActorHasTag` "Reflected") (`self.ActorHasTag` "Thrown")))
    (bind _asbp_dd (cast `/Game/Game/Characters/DD/BP_DD` (`GameplayStatics.GetPlayerCharacter` 0)))
    (bind (_returnvalue_x_2 _returnvalue_y_2) (`KismetMathLibrary.BreakVector` (`SceneComponent.K2_GetComponentLocation` (`/Game/Game/Characters/DD/BP_DD.Pointer` _asbp_dd))))
    (`SceneComponent.K2_SetWorldLocation` (`self.Cube`) (`KismetMathLibrary.MakeVector` _returnvalue_x_2 _returnvalue_y_2 _returnvalue_z) false false)))

(event `self.ReceiveAnyDamage`
  (params (Damage :type "Float (single-precision)") (DamageType :type "DamageType Object Reference") (InstigatedBy :type "Controller Object Reference") (DamageCauser :type "Actor Object Reference"))
  (`/Engine/EditorBlueprintResources/StandardMacros.IsValid` DamageCauser
    (:`Is Valid`
      (if (`self.ActorHasTag` DamageCauser "Player")
        (`self.Reflect` DamageCauser)))))

(fn `Reflect`
  (params (DamageCauser :type "Actor Object Reference"))
  (set `MovementComponent.Velocity` (* (+ (`self.GetActorForwardVector` DamageCauser) (0.0 0.0 0.2)) 1800.0) (`self.ProjectileMovement`))
  (`parent.Reflect` DamageCauser))

(fn `UserConstructionScript`)