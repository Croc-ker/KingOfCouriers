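; BP_DDEncoreBat is a spinning bat projectile that damages actors tagged Enemy and ricochets between them.
; Each enemy overlap applies damage, plays a hit sound and increments a bounce counter, destroying the bat at BounceMax.
; Before that limit, it waits a tick, then redirects ProjectileMovement at max speed toward the nearest tagged enemy within range, without excluding the one just hit.
; Tick spins the mesh by a fixed, frame-rate-dependent step.
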(event `self.ReceiveActorBeginOverlap`
  (params (OtherActor :type "Actor Object Reference"))
  (bind _projectilemovement (`self.ProjectileMovement`))
  (`/Engine/EditorBlueprintResources/StandardMacros.IsValid` OtherActor
    (:`Is Valid`
      (if (`self.ActorHasTag` OtherActor "Enemy")
        (`GameplayStatics.ApplyDamage` OtherActor 200.0)
        (`GameplayStatics.PlaySoundAtLocation` "/Game/Game/Sounds/physical/Bat-Hit.Bat-Hit" (`self.K2_GetActorLocation`) (struct) 1.0 1.0 0.0 null null self null)
        (bind _result (`/Engine/EditorBlueprintResources/StandardMacros.IncrementInt` (`self.BounceIndex`))
          (:`  `
            (if (< _result (`self.BounceMax`))
              (`KismetSystemLibrary.DelayUntilNextTick`)
              (bind _outactors (`GameplayStatics.GetAllActorsWithTag` "Enemy"))
              (bind (_distance _returnvalue) (`GameplayStatics.FindNearestActor` (`self.K2_GetActorLocation`) _outactors))
              (if (and (<= _distance 1000.0) (`KismetSystemLibrary.IsValid` _returnvalue))
                (set `MovementComponent.Velocity` (* (`KismetMathLibrary.GetForwardVector` (`KismetMathLibrary.FindLookAtRotation` (`self.K2_GetActorLocation`) (`self.K2_GetActorLocation` _returnvalue))) (`ProjectileMovementComponent.MaxSpeed` _projectilemovement)) _projectilemovement))
              (else
                (`self.K2_DestroyActor`)))))))))

(event `self.ReceiveTick`
  (params (DeltaSeconds :type "Float (single-precision)"))
  (`SceneComponent.K2_AddRelativeRotation` (`self.StaticMesh`) (struct :`Yaw` 25.0) false false))

(fn `UserConstructionScript`)